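; Behavior tree task that sets a patrolling AI's next Waypoint in the Blackboard, then finishes successfully.
; It writes the TargetLocations entry at the stored Index to Waypoint.
; It then stores a random Index, or the next wrapped one when a random roll matches the current.
; GetPatrolPoints only casts the pawn to BP_TG_AI; its copy of PatrolPoints into TargetLocations is disconnected.
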(event `self.ReceiveExecuteAI`
  (params (OwnerController :type "AIController Object Reference") (ControlledPawn :type "Pawn Object Reference"))
  (`self.GetPatrolPoints` ControlledPawn)
  (bind _index (`self.SetNextWaypoint`))
  (`self.SycleIndex` _index)
  (`self.FinishExecute` true))

(fn `GetPatrolPoints`
  (params (Object :type "Object Object Reference"))
  (cast `/Game/Project/P4/AI/BP_TG_AI` Object))

(fn `SetNextWaypoint`
  (returns (Index :type Integer))
  (bind _returnvalue (`BTFunctionLibrary.GetBlackboardValueAsInt` (`self.Index`)))
  (`BTFunctionLibrary.SetBlackboardValueAsObject` (`self.Waypoint`) (`|GetArrayItem` (`self.TargetLocations`) _returnvalue))
  (return _returnvalue))

(fn `SycleIndex`
  (params (CurrentIndex :type Integer))
  (bind _returnvalue (`KismetArrayLibrary.Array_Length` (`self.TargetLocations`)))
  (bind _returnvalue_2 (`KismetMathLibrary.RandomIntegerInRange` 0 (- _returnvalue 1)))
  (`BTFunctionLibrary.SetBlackboardValueAsInt` (`self.Index`) (`KismetMathLibrary.SelectInt` (mod (+ CurrentIndex 1) _returnvalue) _returnvalue_2 (== CurrentIndex _returnvalue_2))))