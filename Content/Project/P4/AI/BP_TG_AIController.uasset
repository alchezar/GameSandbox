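; AI controller for a guard character, running the guard behavior tree on the patrol blackboard.
; Perception updates store any sensed actor without the Bot tag as the Enemy key.
; Any other update, including a lost target or a sensed bot, clears Enemy and sets the character's aiming state by whether LastSeenLocation is set.
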(event `self.ReceiveBeginPlay`
  (bind _blackboardcomponent (`self.UseBlackboard` "/Game/Project/P4/AI/BB_TG_PatrolData.BB_TG_PatrolData"))
  (set `self.Blackboard Comp` _blackboardcomponent)
  (`self.RunBehaviorTree` "/Game/Project/P4/AI/BT_GuardBehavior.BT_GuardBehavior")
  (bind _astg_base_character (cast `TG_BaseCharacter` (`self.K2_GetPawn`)))
  (set `self.Base Character` _astg_base_character))

(event `self.AIPerception.OnTargetPerceptionUpdated`
  (params (Actor :type "Actor Object Reference") (Stimulus :type "AIStimulus Structure"))
  (bind _blackboard_comp (`self.Blackboard Comp`))
  ;[0 0 0] Update enemy key
  (if (and (`.bSuccessfullySensed` (break `AIStimulus` Stimulus)) (not (`self.ActorHasTag` Actor "Bot")))
    (`BlackboardComponent.SetValueAsObject` _blackboard_comp "Enemy" Actor)
    (else
      (`BlackboardComponent.ClearValue` _blackboard_comp "Enemy")
      (`TG_BaseCharacter.SetIsAiming` (`self.Base Character`) (`BlackboardComponent.IsVectorValueSet` (`self.Blackboard Comp`) "LastSeenLocation")))))

(fn `UserConstructionScript`)