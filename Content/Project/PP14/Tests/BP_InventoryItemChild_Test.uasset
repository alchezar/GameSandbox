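; BP_InventoryItemChild_Test is a test child Blueprint of an inventory item, inheriting its construction script from the parent.
; SetInventoryData stores the incoming inventory data and passes the color to InitItem.
; SetTestData formats int, float, string, bool and vector inputs into one debug string and prints it on screen.
; BeginPlay, overlap and Tick are disabled placeholder nodes.
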(event `SetTestData`
  (params (Int :type Integer) (Float :type "Float (double-precision)") (String :type String) (Bool :type Boolean) (Vector :type "Vector Structure"))
  (`KismetSystemLibrary.PrintString` (`KismetTextLibrary.Conv_TextToString` (`|FormatText` "Int: {Int} \nFloat: {Float} \nString: {String} \nBool: {Bool} \nVector: {Vector}" Int Float String Bool (`KismetStringLibrary.Conv_VectorToString` Vector))) true true (struct :`G` 0.66 :`B` 1.0 :`A` 1.0) 10.0))

(event `SetInventoryData`
  (params (Data :type "P14InventoryData Structure") (Color :type "LinearColor Structure"))
  (set `self.InventoryData` Data)
  (`self.InitItem` Color))

(fn `UserConstructionScript`
  (`parent.UserConstructionScript`))