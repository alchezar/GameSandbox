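; BP_TEST_Blackhole is a test black hole actor that applies radial gravity to nearby physics objects and consumes them.
; While Active, Tick applies a mass-independent radial force to simulating components overlapping Sphere, whose radius the construction script sets from Radius.
; Each overlap with a second sphere, Sphere1, shrinks the actor and applies a weaker radial impulse, or destroys it once its smallest scale axis drops below half.
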(event `self.ReceiveTick`
  (params (DeltaSeconds :type "Float (single-precision)"))
  (for _array_element (`PrimitiveComponent.GetOverlappingComponents` (`self.Sphere`))
    (if (`self.bActive`)
      (if (`SceneComponent.IsSimulatingPhysics` _array_element "None")
        (`PrimitiveComponent.AddRadialForce` _array_element (`self.K2_GetActorLocation`) (`self.Radius`) (`self.Gravitation`) "RIF_Constant" true)))))

(event `self.Sphere1.OnComponentBeginOverlap`
  (params (OverlappedComponent :type "PrimitiveComponent Object Reference") (OtherActor :type "Actor Object Reference") (OtherComp :type "PrimitiveComponent Object Reference") (OtherBodyIndex :type Integer) (bFromSweep :type Boolean) (SweepResult :type "HitResult Structure (by ref)"))
  (bind _returnvalue (`self.GetActorScale3D` OtherActor))
  (if (< (`KismetMathLibrary.GetMinElement` _returnvalue) 0.5)
    (`self.K2_DestroyActor` OtherActor)
    (else
      (`self.SetActorScale3D` OtherActor (* _returnvalue 0.9))
      (`PrimitiveComponent.AddRadialImpulse` OtherComp (`self.K2_GetActorLocation`) (`self.Radius`) (* (`self.Gravitation`) 0.1) "RIF_Constant" true))))

(fn `UserConstructionScript`
  (`SphereComponent.SetSphereRadius` (`self.Sphere`) (`self.Radius`) true))