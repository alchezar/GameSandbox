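; Enemy AI controller that runs a behavior tree and feeds it perception results about the player.
; Perception updates track one sensed actor tagged Player and branch by sense: sight sets the target actor and visibility flag, while hearing and damage record only a last known location.
; Losing the stimulus stores that actor's current location as the last known one and clears the tracked actor.
; A shared function overwrites all target Blackboard keys on each update.
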(event `self.ReceiveBeginPlay`
  (`self.RunBehaviorTree` (`self.BehaviorTree`)))

(event `self.AIPerception.OnTargetPerceptionUpdated`
  (params (Actor :type "Actor Object Reference") (Stimulus :type "AIStimulus Structure"))
  (bind _seenactor (`self.SeenActor`))
  (if (and (`KismetSystemLibrary.IsValid` _seenactor) (== _seenactor Actor))
    ;[0 0 0] Clear values
    (if (`.bSuccessfullySensed` (break `AIStimulus` Stimulus))
      (`self.SetKeysBySence` Stimulus :!label _label)
      (else
        (`self.SetCurrentBlackboardValues` null (`self.K2_GetActorLocation` (`self.SeenActor`)) false true)
        (set `self.SeenActor` null)))
    (elif (and (`self.ActorHasTag` Actor "Player") (`.bSuccessfullySensed` (break `AIStimulus` Stimulus)))
      (set `self.SeenActor` Actor)
      (goto _label))))

(event `SetKeysBySence`
  (params (Stimulus :type "AIStimulus Structure (by ref)"))
  (bind _seenactor (`self.SeenActor`))
  (bind _returnvalue (`AIPerceptionSystem.GetSenseClassForStimulus` Stimulus))
  (if (== _returnvalue "/Script/AIModule.AISense_Sight")
    (`self.SetCurrentBlackboardValues` _seenactor (`self.K2_GetActorLocation` _seenactor) true)
    (elif (== _returnvalue "/Script/AIModule.AISense_Hearing")
      (`self.SetCurrentBlackboardValues` null (`self.K2_GetActorLocation` (`self.SeenActor`)) false true)
      (elif (== _returnvalue "/Script/AIModule.AISense_Damage")
        (`self.SetCurrentBlackboardValues` null (`self.K2_GetActorLocation` (`self.SeenActor`)) false true)))))

(fn `SetCurrentBlackboardValues`
  (params (TargetActor :type "Object Object Reference") (TargetLocation :type "Vector Structure") (bCanSeeActor :type Boolean) (bLastTarget :type Boolean))
  (bind _returnvalue (`AIBlueprintHelperLibrary.GetBlackboard` null))
  (bind _returnvalue_2 (`AIBlueprintHelperLibrary.GetBlackboard` null))
  (`BlackboardComponent.SetValueAsObject` _returnvalue_2 "TargetActor" TargetActor)
  (`BlackboardComponent.SetValueAsVector` _returnvalue_2 "Target" TargetLocation)
  (`BlackboardComponent.SetValueAsBool` _returnvalue_2 "bCanSeeActor" bCanSeeActor)
  (if bLastTarget
    (`BlackboardComponent.SetValueAsVector` _returnvalue "LastTargetLocation" TargetLocation)
    (else
      (`BlackboardComponent.ClearValue` _returnvalue "LastTargetLocation"))))

(fn `UserConstructionScript`)