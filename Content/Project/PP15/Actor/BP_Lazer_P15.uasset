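; BP_Lazer_P15 is a laser skill actor that tracks hostile characters inside its sphere and signals periodic damage for them.
; Sphere overlaps add characters hostile to the instigator to a list and remove them on exit.
; A looping timer sends the instigator a deal-damage gameplay event carrying those targets, the sphere and the interval as magnitude.
; A helper reports the sphere's distance from the actor relative to the original length.
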(event `self.ReceiveBeginPlay`
  (`KismetSystemLibrary.K2_SetTimerDelegate` (delegate `SendDealDamageEvent`) (`self.Frequency`) true))

(event `SendDealDamageEvent`
  (if (not (`KismetArrayLibrary.Array_IsEmpty` (`self.OverlappingActors`)))
    _
    (else
      _))
  (`AbilitySystemBlueprintLibrary.SendGameplayEventToActor` (`self.GetInstigator`) (struct :`TagName` "p15.skill.laser.deal_damage") (make `GameplayEventData` (struct) null null (`self.Sphere`) null (struct) (struct) (struct) (`self.Frequency`) (`AbilitySystemBlueprintLibrary.AbilityTargetDataFromActorArray` (`self.OverlappingActors`)))))

(event `self.Sphere.OnComponentBeginOverlap`
  (params (OverlappedComponent :type "PrimitiveComponent Object Reference") (OtherActor :type "Actor Object Reference") (OtherComp :type "PrimitiveComponent Object Reference") (OtherBodyIndex :type Integer) (bFromSweep :type Boolean) (SweepResult :type "HitResult Structure (by ref)"))
  (bind _asp15character (cast `P15Character` OtherActor))
  (bind _asp15character_2 (cast `P15Character` (`self.GetInstigator`)))
  (if (`P15Character.GetIsHostile` _asp15character_2 _asp15character)
    (`KismetArrayLibrary.Array_AddUnique` (`self.OverlappingActors`) OtherActor)))

(event `self.Sphere.OnComponentEndOverlap`
  (params (OverlappedComponent :type "PrimitiveComponent Object Reference") (OtherActor :type "Actor Object Reference") (OtherComp :type "PrimitiveComponent Object Reference") (OtherBodyIndex :type Integer))
  (if (`KismetArrayLibrary.Array_Contains` (`self.OverlappingActors`) OtherActor)
    (`KismetArrayLibrary.Array_RemoveItem` (`self.OverlappingActors`) OtherActor)))

(fn `GetLaserLengthOffset`
  (returns (Offset :type "Float (double-precision)"))
  (bind _sphere (`self.Sphere`))
  (`/Engine/EditorBlueprintResources/StandardMacros.IsValid` _sphere
    (:`Is Valid`
      (return (- (`KismetMathLibrary.Vector_Distance` (`SceneComponent.K2_GetComponentLocation` _sphere) (`self.K2_GetActorLocation`)) (`self.OriginalLength`))))))

(fn `UserConstructionScript`)