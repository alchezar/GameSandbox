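; BP_Enemy_P15 is an enemy Blueprint for the PP15 project that hooks up a health bar widget to itself.
; On BeginPlay it runs the parent logic, casts its Widget component's widget to P15HealthBarWidget and passes itself through FindOwner.
; Overlap and Tick events are disabled, and the construction script only calls the parent.
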(event `self.ReceiveBeginPlay`
  (`parent.ReceiveBeginPlay`)
  (bind _asp15health_bar_widget (cast `P15HealthBarWidget` (`WidgetComponent.GetWidget` (`self.Widget`))))
  (`P15HealthBarWidget.FindOwner` _asp15health_bar_widget self))

(fn `UserConstructionScript`
  (`parent.UserConstructionScript`))