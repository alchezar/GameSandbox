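; Actor whose mesh fades out and back in when FadeOut or Fadein is called.
; FadeOut lazily creates dynamic copies of the original materials, swaps them in, and reverses a shared timeline that drives their "Fade" parameter.
; Fadein plays that timeline forward and restores the original materials when it finishes.
; With IgnoreWhenInvisible set, the mesh also ignores GameTraceChannel3 while faded, blocking it again afterwards.
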(event `self.ReceiveBeginPlay`
  (set `self.OriginalMaterials` (`MeshComponent.GetMaterials` (`self.Mesh`))))

(event `/Game/Project/PP16/Actors/FadeActor/BI_Fade_P16.FadeOut`
  (if (`KismetArrayLibrary.Array_IsEmpty` (`self.DynamicMaterials`))
    (for _array_element (`self.OriginalMaterials`)
      (bind _returnvalue (`KismetMaterialLibrary.CreateDynamicMaterialInstance` _array_element))
      (`KismetArrayLibrary.Array_Add` (`self.DynamicMaterials`) _returnvalue)))
  (`self.StartFadeOut`))

(event `/Game/Project/PP16/Actors/FadeActor/BI_Fade_P16.FadeIn`
  (`self.StartFadeIn`))

(event `UpdateMaterials`
  (params (NewMaterials :type "Array of MaterialInterface Object Reference"))
  (for (_array_element _array_index) NewMaterials
    (`PrimitiveComponent.SetMaterial` (`self.Mesh`) _array_index _array_element)))

(event `UpdateFadeAmount`
  (params (FadeAmount :type "Float (single-precision)"))
  (for _array_element (`self.DynamicMaterials`)
    (`MaterialInstanceDynamic.SetScalarParameterValue` _array_element "Fade" FadeAmount)))

(event `StartFadeIn`
  (bind (_direction _fadeamount) (`Timeline|FadeTimeline` :!via `PlayFromStart` :!label _label)
    (:`Update`
      (`self.UpdateFadeAmount` _fadeamount))
    (:`Finished`
      (if (>= _fadeamount (`TimelineComponent.GetTimelineLength` (`self.FadeTimeline`)))
        (`self.AfterFadeIn`)))))

(event `StartFadeOut`
  (`self.BeforeFadeOut`)
  (goto _label :!via `ReverseFromEnd`))

(event `BeforeFadeOut`
  (`self.UpdateMaterials` (`self.DynamicMaterials`))
  (if (`self.bIgnoreWhenInvisible`)
    (`PrimitiveComponent.SetCollisionResponseToChannel` (`self.Mesh`) "ECC_GameTraceChannel3" "ECR_Ignore")))

(event `AfterFadeIn`
  (`self.UpdateMaterials` (`self.OriginalMaterials`))
  (if (`self.bIgnoreWhenInvisible`)
    (`PrimitiveComponent.SetCollisionResponseToChannel` (`self.Mesh`) "ECC_GameTraceChannel3" "ECR_Block")))

(fn `UserConstructionScript`)