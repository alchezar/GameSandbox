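; Fire Blast ball actor that flies outward, then returns to its instigator like a boomerang.
; On BeginPlay, only the authority runs an outgoing timeline that lerps its location from Start to End.
; A returning timeline then lerps from End to the instigator's current location, re-read each update to track movement.
; Once within ExplodeDistance of the instigator, it stops that timeline and destroys itself.
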(event `self.ReceiveBeginPlay`
  (`self.StartTimeline`))

(event `StartTimeline`
  (`/Engine/EditorBlueprintResources/ActorMacros.Switch Has Authority`
    (:`Authority`
      (bind (_direction _alpha) (`Timeline|OutgoingTimeline` :!via `PlayFromStart`)
        (:`Update`
          (`self.K2_SetActorLocation` (`KismetMathLibrary.VLerp` (`self.Start`) (`self.End`) _alpha)))
        (:`Finished`
          (bind (_direction_2 _alpha_2) (`Timeline|ReturningTimeline` :!via `PlayFromStart` :!label _label)
            (:`Update`
              (`self.K2_SetActorLocation` (`KismetMathLibrary.VLerp` (`self.End`) (`self.K2_GetActorLocation` (`self.GetInstigator`)) _alpha_2))
              (if (<= (`KismetMathLibrary.Vector_Distance` (`self.K2_GetActorLocation`) (`self.K2_GetActorLocation` (`self.GetInstigator`))) (`self.ExplodeDistance`))
                (`self.StopReturning`)
                (`self.K2_DestroyActor`)))))))))

(event `StopReturning`
  (goto _label :!via `Stop`))

(fn `UserConstructionScript`)